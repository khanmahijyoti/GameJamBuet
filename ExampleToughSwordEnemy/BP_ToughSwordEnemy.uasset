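; Tough sword enemy Blueprint that adds weapon, health bar and equipment-drop behavior on top of its parent class.
; On begin play it registers the weapon mesh's sockets with the collision component as a main-weapon melee trace target.
; Combat toggles move the weapon between held and sheathed spear sockets, and the health widget binds to the attributes component.
; Dropping equipment briefly waits, then detaches the weapon as a physics-simulated ragdoll object.
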(event OnCombatToggled(CombatComponent)
  (params (bCombatEnabled? :type Boolean))
  (Transformation|AttachComponentToComponent (Variables|Default|GetWeapon%20Mesh) (Variables|Character|GetMesh) (select bCombatEnabled? "SpearSocket" "SpearSocketSheathe") "SnapToTarget" "SnapToTarget" "SnapToTarget" true))

(event EventBeginPlay
  (bind _weapon_mesh (Variables|Default|GetWeapon%20Mesh))
  (|CallParentFunction)
  (bind _returnvalue (Default|AddCollisionTargetType (Variables|Default|GetCollisionComponent) "(TagName=\"TargetType.MainWeapon\")" "/Game/AdvancedARPGCombat/AdvancedCombatFramework/CoreCombatSystem/Actors/CollisionTargetTypes/BP_EnemyMeleeAbilityTraceTarget.BP_EnemyMeleeAbilityTraceTarget_C" self))
  (Default|SetCollisionProperties _returnvalue _weapon_mesh (Transformation|GetAllSocketNames _weapon_mesh)))

(event EventInitializeHUD
  (params (CombatTarget :type Actor%20Object%20Reference))
  (bind _asenemy_health (Utilities|Casting|CastToEnemyHealth (UserInterface|GetUserWidgetObject (Variables|Default|GetHealthBarWidget))))
  (Default|InitializeStatBars _asenemy_health (Variables|Default|GetAttributesComponent)))

(event EventDropEquipment
  (bind _weapon_mesh (Variables|Default|GetWeapon%20Mesh))
  (Utilities|FlowControl|Delay 0.2)
  (Transformation|DetachFromComponent (Variables|Default|GetWeapon%20Mesh) "KeepWorld" "KeepWorld" "KeepWorld" true)
  (Collision|SetCollisionEnabled (Variables|Default|GetWeapon%20Mesh) "QueryAndPhysics")
  (Physics|SetSimulatePhysics _weapon_mesh true)
  (Collision|SetCollisionProfileName _weapon_mesh "ragdoll" true :!class /Script/Engine.PrimitiveComponent))

(fn ConstructionScript
  (|CallParentFunction))